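; Player pawn that moves on forward/right axis input and is meant to count coins it touches.
; Axis events add movement input along actor vectors scaled by MaxSpeed.
; Tick consumes that world-space vector and applies it as a swept, delta-time-scaled local offset, without using a movement component.
; Cube overlap increments NowCoins when OverlappedComponent, the pawn's own component rather than the other actor, equals BP_Coin.
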(event OnComponentBeginOverlap(Cube)
  (params (OverlappedComponent :type Primitive%20Component%20Object%20Reference) (OtherActor :type Actor%20Object%20Reference) (OtherComp :type Primitive%20Component%20Object%20Reference) (OtherBodyIndex :type Integer) (bFromSweep :type Boolean) (SweepResult :type Hit%20Result%20Structure%20%28by%20ref%29))
  (if (== OverlappedComponent "/Game/Object/Collectables/BP_Coin.BP_Coin")
    (Variables|Default|SetNowCoins (+ (Variables|Default|GetNowCoins) 1))))

(event EventTick
  (params (DeltaSeconds :type Float%20%28single-precision%29))
  (bind _returnvalue (Class|Pawn|ConsumeMovementInputVector))
  (Transformation|AddActorLocalOffset (* _returnvalue DeltaSeconds) true false))

(event Input|AxisEvents|InputAxisMoveForward
  (params (AxisValue :type Float%20%28single-precision%29))
  (Pawn|Input|AddMovementInput (Transformation|GetActorForwardVector) (* (Variables|Default|GetMaxSpeed) AxisValue) false))

(event Input|AxisEvents|InputAxisMoveRight
  (params (AxisValue :type Float%20%28single-precision%29))
  (Pawn|Input|AddMovementInput (Transformation|GetActorRightVector) (* AxisValue (Variables|Default|GetMaxSpeed)) false))

(fn ConstructionScript)